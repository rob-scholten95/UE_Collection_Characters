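; Pawn for a simple RTS-style camera with movement, stepped yaw rotation and zoom.
; BeginPlay adds the RTS input mapping context and starts the spring arm at half the maximum zoom.
; Enhanced Input actions pass tunable speed, limit and inversion settings to shared move, rotate and zoom calls.
; Rotation steps once per press, while zoom works on the spring arm with optional pitch adjustment.
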(event Input|EnhancedActionEvents|EnhancedInputActionIA_RTS_Move
  (params (ActionValue :type Vector%202D%20Structure) (ElapsedSeconds :type Float%20%28double-precision%29) (TriggeredSeconds :type Float%20%28double-precision%29) (InputAction :type Input%20Action%20Object%20Reference :default "/Game/Project/02_RTS-Simple/Input/IA_RTS_Move.IA_RTS_Move"))
  (CallFunction|MoveCharacter (.x ActionValue) (.y ActionValue) (Variables|Move|GetInverse%20X) (Variables|Move|GetInverse%20Y) (Variables|Move|GetMovement%20Speed)))

(event Input|EnhancedActionEvents|EnhancedInputActionIA_RTS_RotateYaw
  (params (ActionValue :type Float%20%28double-precision%29) (ElapsedSeconds :type Float%20%28double-precision%29) (TriggeredSeconds :type Float%20%28double-precision%29) (InputAction :type Input%20Action%20Object%20Reference :default "/Game/Project/02_RTS-Simple/Input/IA_RTS_RotateYaw.IA_RTS_RotateYaw"))
  (:Started
    (CallFunction|RotateCameraYaw ActionValue (Variables|Rotate|GetRotate%20Increment) (Variables|Rotate|GetInverse))))

(event Input|EnhancedActionEvents|EnhancedInputActionIA_RTS_Zoom
  (params (ActionValue :type Float%20%28double-precision%29) (ElapsedSeconds :type Float%20%28double-precision%29) (TriggeredSeconds :type Float%20%28double-precision%29) (InputAction :type Input%20Action%20Object%20Reference :default "/Game/Project/02_RTS-Simple/Input/IA_RTS_Zoom.IA_RTS_Zoom"))
  (CallFunction|ZoomCamera ActionValue (Variables|Zoom|GetMinimum%20Zoom) (Variables|Zoom|GetMaximum%20Zoom) (Variables|Zoom|GetZoom%20Speed) (Variables|Default|GetSpringArm) (Variables|Pitch|GetZoom%20Pitch%20Inverse) 1e+02 (Variables|Pitch|GetZoom%20Pitch%20Enabled)))

(event EventBeginPlay
  (CallFunction|AddMappingContext "/Game/Project/02_RTS-Simple/Input/IMC_RTS_Default.IMC_RTS_Default")
  ;[1 1 1] Comment
  (Variables|/Script/Engine.SpringArmComponent|SetTargetArmLength (Variables|Default|GetSpringArm) (/ (Variables|Zoom|GetMaximum%20Zoom) 2.0)))

(event Collision|EventActorBeginOverlap
  (params (OtherActor :type Actor%20Object%20Reference)))

(event EventTick
  (params (DeltaSeconds :type Float%20%28single-precision%29)))

(fn ConstructionScript)