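; Actor component that switches the player to another pawn dropped at the mouse cursor location.
; InitComponent spawns a BP_DropPin, which a looping timer, used instead of Tick, keeps under the cursor or hides far below on a miss.
; Click-Completed replaces existing pawns of the target class with one at the cursor, removes pin and timer, then blends the view over and possesses it after the blend delay.
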(event Custom|CustomTick
  (bind _array (Utilities|Array|MakeArray "ObjectTypeQuery1"))
  (bind _droppin (Variables|Default|GetDropPin))
  (bind _data (CallFunction|GetHitResultCursor _array))
  (bind (_bblockinghit _binitialoverlap _time _distance _location) (Collision|BreakHitResult _data))
  (Utilities|IsValid (Variables|Default|GetDropPin)
    (:Is%20Valid
      ;[1 1 1] Set Pin To Cursor Location
      (if _bblockinghit
        (bind _output_get (Variables|Default|SetCursorLocation (+ _location "0.000000,0.000000,5.000000")))
        ;;[1 1 1] If Hit, Set to HitLocation
        (Transformation|SetActorLocation _droppin _output_get false false)
        (else
          ;;[1 1 1] If Not Hit, set far away
          (Transformation|SetActorLocation _droppin "0.000000,0.000000,-999999.000000" false false))))))

(event Custom|InitComponent
  (bind _array (Utilities|Array|MakeArray "ObjectTypeQuery1"))
  (bind (_ishit _data) (CallFunction|GetHitResultCursor _array))
  (Utilities|FlowControl|Sequence
    (:then_0
      ;[1 1 1] Get and Set owner
      (Variables|Default|SetOwner (Components|GetOwner)))
    (:then_1
      ;[1 1 1] Create Drop Pin At Mouse Location
      (if _ishit
        (bind _returnvalue (Game|SpawnActorfromClass "/Game/Project/Components/SwitchPawns/Pin/BP_DropPin.BP_DropPin_C" (Math|Conversions|ToTransform(Vector) (.Location (Collision|BreakHitResult _data))) "Undefined" "MultiplyWithRoot" 0 0))
        (Variables|Default|SetDropPin _returnvalue)))
    (:then_2
      ;[1 1 1] Start Custom Tick Event for Performance
      (bind _returnvalue_2 (Utilities|Time|SetTimerbyEvent (EventDispatchers|CreateEvent :!event Custom|CustomTick) 0.01 true))
      (Variables|Default|SetCustomTickTimer _returnvalue_2))))

(event Custom|Click-Completed
  ;[1 1 1] OnReleasingMouseButton
  (Utilities|FlowControl|Sequence
    (:then_0
      ;[1 1 1] If A pawn already exists in the scene, delete it to avoid confusion
      (bind _outactors (Actor|GetAllActorsOfClass (Variables|Default|GetPawnToSwitchToClass)))
      (for _array_element _outactors
        (Actor|DestroyActor _array_element))
      (Variables|Default|SetPawnToSwitchTo 0))
    (:then_1
      ;[1 1 1] Spawn new Pawn at Cursor location
      (bind _returnvalue (Game|SpawnActorfromClass (Variables|Default|GetPawnToSwitchToClass) (Math|Conversions|ToTransform(Vector) (Variables|Default|GetCursorLocation)) "Undefined" "MultiplyWithRoot" 0 0))
      (Variables|Default|SetPawnToSwitchTo _returnvalue)
      ;[1 1 1] If exists, Destroy DropPin Actor
      (Utilities|IsValid (Variables|Default|GetDropPin)
        (:Is%20Valid
          (Actor|DestroyActor (Variables|Default|GetDropPin))
          (Variables|Default|SetDropPin 0)
          (Variables|Default|SetCursorLocation "0, 0, 0"))
        (:Is%20Not%20Valid
          _))
      ;[1 1 1] Clear timer for CustomTick
      (Utilities|Time|ClearandInvalidateTimerbyHandle (Variables|Default|GetCustomTickTimer)))
    (:then_2
      ;[1 1 1] Switch to other pawn using View Target Blend and Possess
      (Game|Player|SetViewTargetwithBlend (Game|GetPlayerController 0) (Variables|Default|GetPawnToSwitchTo) 1.5 "VTBlend_EaseInOut" 1.0 false)
      (Utilities|FlowControl|Delay 1.5)
      (Pawn|Possess (Game|GetPlayerController 0) (Variables|Default|GetPawnToSwitchTo))
      (Variables|Default|SetIsSwitchedToOtherPawn true))))

(fn GetHitResultCursor
  (params (ObjectTypes :type Array%20of%20EObjectTypeQuery%20Enums :default "ObjectTypeQuery1"))
  (bind _returnvalue (Game|GetPlayerController 0))
  (bind _hitresult (Class|PlayerController|GetHitResultUnderCursorforObjects _returnvalue ObjectTypes true))
  (bind _bblockinghit (Collision|BreakHitResult _hitresult))
  (if _bblockinghit
    (return _bblockinghit _hitresult)))