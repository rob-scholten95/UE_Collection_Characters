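; Blueprint function library for touch camera control, with orbit and pinch zoom helpers for player 0.
; TouchOrbit turns the end-to-start screen position ratio into invertible control rotation changes, clamping pitch to hardcoded limits (PitchMin/PitchMax are unused), and returns the end location.
; GetTouchDistance measures the gap between two fingers, substituting mouse position length on Windows.
; TouchPinch eases spring arm length toward a supplied distance using delta-time-scaled Lerp.
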(fn TouchOrbit
  (params (StartLocation :type Vector%202D%20Structure) (EndLocation :type Vector%202D%20Structure) (Invert%20Yaw? :type Boolean) (Invert%20Pitch? :type Boolean) (RotationSpeedTouch :type Float%20%28double-precision%29) (Pitch%20Min :type Float%20%28double-precision%29) (Pitch%20Max :type Float%20%28double-precision%29))
  (bind _returnvalue (Game|GetPlayerController 0))
  (bind _returnvalue_2 (Pawn|GetControlRotation _returnvalue :!class /Script/Engine.Controller))
  (Pawn|SetControlRotation (Game|GetPlayerController 0) (Math|Rotator|MakeRotator 0.0 (Math|Float|ClampAngle (+ (.pitch _returnvalue_2) (* (* (- (/ (.y EndLocation) (.y StartLocation)) 1.0) -1.0) (Math|Float|SelectFloat (* -1 RotationSpeedTouch) RotationSpeedTouch Invert%20Pitch?))) -9e+01 5.0) (+ (* (- (/ (.x EndLocation) (.x StartLocation)) 1.0) (Math|Float|SelectFloat (* -1 RotationSpeedTouch) RotationSpeedTouch Invert%20Yaw?)) (.yaw _returnvalue_2))))
  (return EndLocation))

(fn GetTouchInput
  (params (FingerIndex :type ETouchIndex%20Enum :default "Touch1"))
  (bind _returnvalue (Game|GetPlayerController 0))
  (bind (_locationx _locationy) (Class|PlayerController|GetInputTouchState _returnvalue FingerIndex))
  (return (Math|Vector2D|MakeVector2D _locationx _locationy)))

(fn GetTouchDistance
  (bind _returnvalue (Game|GetPlayerController 0))
  (bind (_locationx _locationy) (Game|Player|GetMousePosition _returnvalue))
  (return (Math|Vector2D|Vector2DLength (select (Utilities|Enum|Equal(Enum) (Game|GetPlatformName) "Windows") (Math|Vector2D|MakeVector2D _locationx _locationy) (- (Utilities|GetTouchInput "Touch1") (Utilities|GetTouchInput "Touch2"))))))

(fn TouchPinch
  (params (Distance :type Float%20%28double-precision%29) (Spring%20Arm :type Spring%20Arm%20Component%20Object%20Reference) (ZoomSpeed :type Float%20%28double-precision%29))
  (Variables|/Script/Engine.SpringArmComponent|SetTargetArmLength Spring%20Arm (Math|Float|Lerp (Variables|/Script/Engine.SpringArmComponent|GetTargetArmLength Spring%20Arm) Distance (* (Utilities|Time|GetWorldDeltaSeconds) ZoomSpeed))))