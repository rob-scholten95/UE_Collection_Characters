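; Touch-testing pawn for an orbit camera, with one-finger orbit, two-finger pinch zoom on a spring arm, and debug-printed single and double taps.
; Enhanced Input actions are gated by a finger count from Touch1–3 presses, with releases delayed briefly.
; A looping timer slowly yaws the control rotation once the idle threshold passes, and touch input resets it.
; The single-tap TapTimer workaround's increment is disconnected.
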(event Custom|Idle
  ;[1 1 1] Idle
  (CallFunction|IdleRotation (Variables|Idle|GetIdle%20Threshold) (Variables|Idle|GetIdle%20Rotation%20Speed) (Variables|Debug|GetDebug%20Idle%20Timer)))

(event Custom|ResetIdle
  ;[1 1 1] Idle
  (Variables|Idle|SetIdleTimer 0.0))

(event Input|EnhancedActionEvents|EnhancedInputActionIA_Touch_Orbit
  (params (ActionValue :type Boolean) (ElapsedSeconds :type Float%20%28double-precision%29) (TriggeredSeconds :type Float%20%28double-precision%29) (InputAction :type Input%20Action%20Object%20Reference :default "/Game/Project/05_Touch_Orbit/Input/Actions/IA_Touch_Orbit.IA_Touch_Orbit"))
  ;[0.5 1 0.5] TOUCH_MOVEMENT
  ;;[1 1 1] TOUCH_ORBIT
  (:Triggered
    (if (== (Variables|AmountOfFingers|GetTouch_F_Count) 1)
      (Variables|FingerInfo|SetEndLocation (CallFunction|GetTouchInput "Touch1"))
      (bind _start_location (CallFunction|TouchOrbit (Variables|FingerInfo|GetStartLocation) (Variables|FingerInfo|GetEndLocation) false false (Variables|Orbit|GetRotation%20Speed%20Touch) (Variables|Orbit|GetPitch%20Min) (Variables|Orbit|GetPitch%20Max)))
      (Variables|FingerInfo|SetStartLocation _start_location)))
  (:Started
    (Variables|FingerInfo|SetStartLocation (CallFunction|GetTouchInput "Touch1"))
    (CallFunction|ResetIdle)))

(event Input|EnhancedActionEvents|EnhancedInputActionIA_Touch_Pinch
  (params (ActionValue :type Boolean) (ElapsedSeconds :type Float%20%28double-precision%29) (TriggeredSeconds :type Float%20%28double-precision%29) (InputAction :type Input%20Action%20Object%20Reference :default "/Game/Project/05_Touch_Orbit/Input/Actions/IA_Touch_Pinch.IA_Touch_Pinch"))
  (bind _usemiddlemouseforzoom (Variables|Debug|GetUseMiddleMouseForZoom))
  (bind _touch_f_count (Variables|AmountOfFingers|GetTouch_F_Count))
  (bind _returnvalue (== _touch_f_count 2))
  (bind _returnvalue_2 (or _returnvalue _usemiddlemouseforzoom))
  ;[0.5 1 0.5] TOUCH_MOVEMENT
  ;;[1 1 1] TOUCH_PINCH TO ZOOM
  (:Triggered
    (CallFunction|ResetIdle)
    (if _returnvalue_2
      (CallFunction|TouchPinch (stale _returnvalue_3) (Variables|Default|GetSpringArm) (Variables|Zoom|GetZoomSpeed))))
  (:Started
    (if _returnvalue_2
      (bind _returnvalue_3 (Utilities|PinchCameraZoom)))))

(event Input|EnhancedActionEvents|EnhancedInputActionIA_Touch_Tap
  (params (ActionValue :type Boolean) (ElapsedSeconds :type Float%20%28double-precision%29) (TriggeredSeconds :type Float%20%28double-precision%29) (InputAction :type Input%20Action%20Object%20Reference :default "/Game/Project/05_Touch_Orbit/Input/Actions/IA_Touch_Tap.IA_Touch_Tap"))
  ;[0.5 1 0.5] TOUCH TAP
  ;;[1 1 1] TOUCH_SINGLETAP
  (:Triggered
    (CallFunction|ResetIdle))
  (:Completed
    (if (== (Variables|AmountOfFingers|GetTouch_F_Count) 1)
      ;;;[1 1 1] Workaround because of bug in when adding triggers to input.
      (if (> (Variables|Default|GetTapTimer) 0.25)
        (Variables|Default|SetTapTimer 0.0)
        (else
          (Variables|Default|SetTapTimer 0.0)
          (if (Variables|Debug|GetDebug%20Tap%20Prints)
            (Development|PrintString "Tap 1x" true true "(R=0.077461,G=1.000000,B=0.000000,A=1.000000)" 1.0)))))))

(event Input|EnhancedActionEvents|EnhancedInputActionIA_Touch_DoubleTap
  (params (ActionValue :type Boolean) (ElapsedSeconds :type Float%20%28double-precision%29) (TriggeredSeconds :type Float%20%28double-precision%29) (InputAction :type Input%20Action%20Object%20Reference :default "/Game/Project/05_Touch_Orbit/Input/Actions/IA_Touch_DoubleTap.IA_Touch_DoubleTap"))
  ;[0.5 1 0.5] TOUCH TAP
  ;;[1 1 1] TOUCH_DOUBLETAP
  (:Started
    (CallFunction|ResetIdle))
  (:Completed
    (if (== (Variables|AmountOfFingers|GetTouch_F_Count) 1)
      (if (Variables|Debug|GetDebug%20Tap%20Prints)
        (Development|PrintString "Tap 2x" true false "(R=0.000000,G=1.000000,B=0.003935,A=1.000000)" 1.0)))))

(event EventBeginPlay
  ;[1 1 1] BEGINPLAY
  (CallFunction|AddMappingContext "/Game/Project/05_Touch_Orbit/Input/IMC_Touch_Default.IMC_Touch_Default")
  (Utilities|Time|SetTimerbyEvent (delegate Custom|Idle) 0.1 true))

(event Input|TouchEvents|Touch1
  (params (Key :type Key%20Structure))
  ;[1 0.2971 0.8877] TOUCH_AMOUNT OF FINGERS ON SCREEN
  (:Pressed
    (Variables|AmountOfFingers|SetTouch_F1_Pressed true)
    (bind _output_get (Variables|AmountOfFingers|SetTouch_F_Count (+ (Math|Conversions|ToInteger(Boolean) (Variables|AmountOfFingers|GetTouch_F1_Pressed)) (Math|Conversions|ToInteger(Boolean) (Variables|AmountOfFingers|GetTouch_F2_Pressed)) (Math|Conversions|ToInteger(Boolean) (Variables|AmountOfFingers|GetTouch_F3_Pressed))) :!label _label))
    (CallFunction|ResetIdle)
    (Development|PrintString (Utilities|String|Append "F Count" (Utilities|String|ToString(Integer) _output_get)) (Variables|Debug|GetTouch_F_Count_Debug?) false "(R=0.017206,G=1.000000,B=0.000000,A=1.000000)"))
  (:Released
    (Utilities|FlowControl|RetriggerableDelay 0.15)
    (Variables|AmountOfFingers|SetTouch_F1_Pressed false)
    (goto _label)))

(event Input|TouchEvents|Touch2
  (params (Key :type Key%20Structure))
  ;[1 0.2971 0.8877] TOUCH_AMOUNT OF FINGERS ON SCREEN
  (:Pressed
    (Variables|AmountOfFingers|SetTouch_F2_Pressed true)
    (bind _output_get (Variables|AmountOfFingers|SetTouch_F_Count (+ (Math|Conversions|ToInteger(Boolean) (Variables|AmountOfFingers|GetTouch_F1_Pressed)) (Math|Conversions|ToInteger(Boolean) (Variables|AmountOfFingers|GetTouch_F2_Pressed)) (Math|Conversions|ToInteger(Boolean) (Variables|AmountOfFingers|GetTouch_F3_Pressed))) :!label _label))
    (CallFunction|ResetIdle)
    (Development|PrintString (Utilities|String|Append "F Count" (Utilities|String|ToString(Integer) _output_get)) (Variables|Debug|GetTouch_F_Count_Debug?) false "(R=0.017206,G=1.000000,B=0.000000,A=1.000000)"))
  (:Released
    (Utilities|FlowControl|RetriggerableDelay 0.15)
    (Variables|AmountOfFingers|SetTouch_F2_Pressed false)
    (goto _label)))

(event Input|TouchEvents|Touch3
  (params (Key :type Key%20Structure))
  ;[1 0.2971 0.8877] TOUCH_AMOUNT OF FINGERS ON SCREEN
  (:Pressed
    (Variables|AmountOfFingers|SetTouch_F3_Pressed true)
    (bind _output_get (Variables|AmountOfFingers|SetTouch_F_Count (+ (Math|Conversions|ToInteger(Boolean) (Variables|AmountOfFingers|GetTouch_F1_Pressed)) (Math|Conversions|ToInteger(Boolean) (Variables|AmountOfFingers|GetTouch_F2_Pressed)) (Math|Conversions|ToInteger(Boolean) (Variables|AmountOfFingers|GetTouch_F3_Pressed))) :!label _label))
    (CallFunction|ResetIdle)
    (Development|PrintString (Utilities|String|Append "F Count" (Utilities|String|ToString(Integer) _output_get)) (Variables|Debug|GetTouch_F_Count_Debug?) false "(R=0.017206,G=1.000000,B=0.000000,A=1.000000)"))
  (:Released
    (Utilities|FlowControl|RetriggerableDelay 0.15)
    (Variables|AmountOfFingers|SetTouch_F3_Pressed false)
    (goto _label)))

(fn ConstructionScript)

(fn IdleRotation
  (params (Idle%20Threshold :type Float%20%28double-precision%29) (RotationSpeed :type Float%20%28double-precision%29) (DebugIdleTimer :type Boolean))
  (bind _returnvalue (Game|GetPlayerController 0))
  (bind _returnvalue_2 (Pawn|GetControlRotation _returnvalue :!class /Script/Engine.Controller))
  (if DebugIdleTimer
    (Development|PrintString (Utilities|String|ToString(Float) (Variables|Idle|GetIdleTimer)) true false "(R=0.000000,G=1.000000,B=0.146822,A=1.000000)" 0.1))
  (bind _output_get (Variables|Idle|SetIdleTimer (+ (Variables|Idle|GetIdleTimer) (Utilities|Time|GetWorldDeltaSeconds))))
  (if (> _output_get Idle%20Threshold)
    (Pawn|SetControlRotation (Game|GetPlayerController 0) (Math|Rotator|MakeRotator (.roll _returnvalue_2) (.pitch _returnvalue_2) (+ (.yaw _returnvalue_2) RotationSpeed)))))