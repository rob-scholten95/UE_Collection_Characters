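; Player controller for an architectural visualization app that shows a landing page, then swaps to the HUD on project start.
; Project start also caches the game mode, flying pawn and scene focus markers.
; Toolbar presses store a Function struct, whose camera marker drives a Timeline lerp of pawn location and control rotation.
; The struct's logic actor class toggles or replaces a single active actor; the animated widget-switcher logic is present but unconnected.
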(event Custom|Focus
  (bind _function (Variables|Default|GetFunction))
  (bind _scenecameramarker (Utilities|Struct|BreakS_FunctionInfo _function))
  (bind _output (Utilities|ResolveSoftReference _scenecameramarker))
  ;[0.1765 0.251 0.349] FOCUS
  (Utilities|IsValid _output
    (:Is%20Valid
      (Variables|Focus|SetCurrentFocusMarker _output)
      (Components|Timeline|SetPlayRate (Variables|Default|GetTimeline) (Variables|Focus|GetFocus%20Play%20Rate))
      (bind _alpha (Timeline|Timeline PlayFromStart) ; Focus animation
        (:Update
          (Transformation|SetActorLocation (Variables|References|GetP%20Arch%20Viz%20Flying) (Math|Vector|Lerp(Vector) (Transformation|GetActorLocation (Variables|References|GetP%20Arch%20Viz%20Flying)) (.Location (Math|Transform|BreakTransform (Transformation|GetActorTransform (Variables|Focus|GetCurrentFocusMarker)))) _alpha) false false)
          (Pawn|SetControlRotation (Game|GetPlayerController 0) (Math|Rotator|Lerp(Rotator) (Pawn|GetControlRotation (Game|GetPlayerController 0) :!class /Script/Engine.Controller) (.Rotation (Math|Transform|BreakTransform (Transformation|GetActorTransform (Variables|Focus|GetCurrentFocusMarker)))) _alpha true)))))))

(event Custom|StopFocusAnimation
  (bind _currentfocusmarker (Variables|Focus|GetCurrentFocusMarker))
  (bind _returnvalue (Transformation|GetActorTransform _currentfocusmarker))
  (bind (_location _rotation) (Math|Transform|BreakTransform _returnvalue))
  ;[0.1765 0.251 0.349] FOCUS
  (bind _alpha (Timeline|Timeline Stop) ; Focus animation
    (:Update
      (Transformation|SetActorLocation (Variables|References|GetP%20Arch%20Viz%20Flying) (Math|Vector|Lerp(Vector) (Transformation|GetActorLocation (Variables|References|GetP%20Arch%20Viz%20Flying)) _location _alpha) false false)
      (Pawn|SetControlRotation (Game|GetPlayerController 0) (Math|Rotator|Lerp(Rotator) (Pawn|GetControlRotation (Game|GetPlayerController 0) :!class /Script/Engine.Controller) _rotation _alpha true)))))

(event EventOnButtonPressed
  (params (Tag :type Name :default "None"))
  (bind _uw_landingpage (Variables|References|GetUW_LandingPage))
  ;[1 0.7765 0.1765 1 36] PROJECT START
  (if (== Tag "project-start")
    (Utilities|FlowControl|Sequence
      (:then_0
        ;;[0.07866 0.1124 0.1545] VALIDITY CHECKING
        ;;;[1 1 1] Check GameMode Validitiy
        (bind _asgm_arch_viz_studio (Utilities|Casting|CastToGM_ArchVizStudio (Game|GetGameMode)))
        (Utilities|IsValid _asgm_arch_viz_studio
          (:Is%20Valid
            (Variables|References|SetGM%20Arch%20Viz%20Studio _asgm_arch_viz_studio)
            ;;;[1 1 1] Comment
            (bind _asp_arch_viz_flying (Utilities|Casting|CastToP_ArchViz_Flying (Game|Player|GetPlayerPawn 0)))
            (Utilities|IsValid _asp_arch_viz_flying
              (:Is%20Valid
                (Variables|References|SetP%20Arch%20Viz%20Flying _asp_arch_viz_flying)
                ;;;[1 1 1] Store all Markers in the scene
                (bind _outactors (Actor|GetAllActorsOfClass "/Game/ArchVizStudio/Blueprints/Focus/BP_Focus_Marker.BP_Focus_Marker_C"))
                (if (Utilities|Array|IsEmpty _outactors)
                  (Development|PrintString "No Focus Markers Found in the scene!")
                  (else
                    (Variables|Focus|SetFocusMarkers _outactors))))
              (:Is%20Not%20Valid
                (Development|PrintString "Player Pawn not Valid!"))))
          (:Is%20Not%20Valid
            (Development|PrintString "Not the default GameMode Object!"))))
      (:then_1
        ;;[0.07866 0.1124 0.1545] WIDGETS
        (bind _returnvalue (UserInterface|CreateWidget "/Game/ArchVizStudio/UI/Menus/UW_HUD.UW_HUD_C" (Game|GetPlayerController 0)))
        (Utilities|IsValid _returnvalue
          (:Is%20Valid
            (bind _output_get (Variables|References|SetUW_HUD _returnvalue))
            (UserInterface|Viewport|AddtoViewport _output_get 0)
            (Widget|SetVisibility _output_get "Collapsed")
            (Components|Animation|PlayAnimation _uw_landingpage (Variables|/Game/ArchVizStudio/UI/Menus/UW_LandingPage.UW_LandingPage_C|Getanim_inandout _uw_landingpage) 0.0
              (:Finished
                (Widget|SetVisibility (Variables|References|GetUW_HUD) "Visible")
                (Widget|RemovefromParent (Variables|References|GetUW_LandingPage))))))))))

(event EventBeginPlay
  ;[1 0.7765 0.1765 1 36] LANDINGPAGE
  (Utilities|FlowControl|Sequence
    (:then_0
      ;;[1 1 1] Create and Store HUD and Add to Viewport
      (bind _returnvalue (UserInterface|CreateWidget "/Game/ArchVizStudio/UI/Menus/UW_LandingPage.UW_LandingPage_C" (Game|GetPlayerController 0)))
      (bind _output_get (Variables|References|SetUW_LandingPage _returnvalue))
      (UserInterface|Viewport|AddtoViewport _output_get 0))))

(event EventOnToolbarButtonPressed
  (params (Function :type S%20Function%20Info%20Structure))
  ;[1 1 1] ON TOOLBAR BUTTON PRESSED
  (Variables|Default|SetFunction Function)
  (Default|CursorHasMovedEvent (Variables|References|GetP%20Arch%20Viz%20Flying))
  (CallFunction|Focus)
  (CallFunction|SpawnFunction))

(fn ConstructionScript)

(fn AnalyzeTag
  (params (InName :type Name))
  (bind _returnvalue (Utilities|String|ToString(Name) InName))
  (bind (_lefts _rights) (Utilities|String|Split _returnvalue "-"))
  (bind (_lefts_2 _rights_2) (Utilities|String|Split _rights "-"))
  (return _lefts _lefts_2 _rights_2))

(fn FindFocusMarkerbyTag
  (params (Tag :type Name))
  (for _array_element (Variables|Focus|GetFocusMarkers)
    (if (Actor|ActorHasTag _array_element Tag)
      (LocalVariables|Setvar _array_element)))
  (return (LocalVariables|Getvar)))

(fn IsIndexValid
  (params (A :type Integer))
  (return (<= A (- (Class|WidgetSwitcher|GetNumWidgets (Variables|/Game/ArchVizStudio/UI/Menus/UW_HUD.UW_HUD_C|GetWidgetSwitcher (Variables|References|GetUW_HUD))) 1))))

(fn SpawnFunction
  (if (Utilities|IsValidClass (.LogicActor (Utilities|Struct|BreakS_FunctionInfo (Variables|Default|GetFunction))))
    (Utilities|IsValid (Variables|Default|GetActiveLogicActor)
      (:Is%20Valid
        (if (== (.LogicActor (Utilities|Struct|BreakS_FunctionInfo (Variables|Default|GetFunction))) (Utilities|GetClass (Variables|Default|GetActiveLogicActor)))
          ;[1 1 1] If the New to spawn Logic Actor is the same as the current Logic Actor, then Delete the current Active Logic Actor
          (Actor|DestroyActor (Variables|Default|GetActiveLogicActor))
          (Variables|Default|SetActiveLogicActor 0)
          (else
            ;[1 1 1] If The Logic Actor is Valid, and the New one is not the same as the current one, Destroy the current one and Spawn a new one.
            (Actor|DestroyActor (Variables|Default|GetActiveLogicActor))
            (bind _returnvalue (Game|SpawnActorfromClass (.LogicActor (Utilities|Struct|BreakS_FunctionInfo (Variables|Default|GetFunction))) (Math|Transform|MakeTransform "0, 0, 0" "0, 0, 0" "1.000000,1.000000,1.000000") "Undefined" "MultiplyWithRoot" 0 0))
            (Variables|Default|SetActiveLogicActor _returnvalue))))
      (:Is%20Not%20Valid
        ;[1 1 1] If theres no Logic Actor in the scene, then spawn one.
        (bind _returnvalue_2 (Game|SpawnActorfromClass (.LogicActor (Utilities|Struct|BreakS_FunctionInfo (Variables|Default|GetFunction))) (Math|Transform|MakeTransform "0, 0, 0" "0, 0, 0" "1.000000,1.000000,1.000000") "Undefined" "MultiplyWithRoot" 0 0))
        (Variables|Default|SetActiveLogicActor _returnvalue_2)))
    (else
      (Utilities|IsValid (Variables|Default|GetActiveLogicActor)
        (:Is%20Valid
          (Actor|DestroyActor (Variables|Default|GetActiveLogicActor)))
        (:Is%20Not%20Valid
          _))
      (return))))